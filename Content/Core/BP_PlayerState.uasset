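; Player state for a minigame match, tracking each player's lives, round and match points, readiness and preferred game rule.
; Loading and introduction events set flags and message the GameMode that the player is ready for that phase.
; Rule selection stores the new choice and sends old and new rules to the GameState, using -1 for no selection.
; A reset event restores per-loop values but keeps match points.
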(event EventPSReduceLifes
  ;[0.15 0.15 0.15 0.5] Gameplay Operations
  (Variables|Default|SetLifes (- (Variables|Default|GetLifes) 1)))

(event EventPSFinishedIntroducing
  ;[0.15 0.15 0.15 0.5] Call To GM
  (Variables|Default|SetFinishedIntroducing true)
  (Class|BPIGameplayLoop|GMReadyforPhase(Message) (Game|GetGameMode) "IntroducingMinigame"))

(event EventPSUpdateMatchPoints
  (params (MatchPointsToRecive :type Integer))
  ;[0.15 0.15 0.15 0.5] Gameplay Operations
  (Variables|Default|SetMatchPoints (+ MatchPointsToRecive (Variables|Default|GetMatchPoints))))

(event EventPSPlayerLoaded
  ;[0.15 0.15 0.15 0.5] Call To GM
  (Variables|Default|SetPlayerLoaded true)
  (Class|BPIGameplayLoop|GMReadyforPhase(Message) (Game|GetGameMode) "WaitingPlayers"))

(event EventPSDefinePreferRuleSelected
  (params (GameRule%20Selected :type Integer))
  (CallFunction|DefinePreferRule GameRule%20Selected))

(event EventDefineLifesValue
  (params (NewLifes :type Integer))
  ;[0.15 0.15 0.15 0.5] Gameplay Operations
  (Variables|Default|SetLifes NewLifes))

(event EventWinRound
  ;[0.15 0.15 0.15 0.5] Gameplay Operations
  (Variables|Default|SetRoundPoints (+ (Variables|Default|GetRoundPoints) 1)))

(event EventPSResetGameloop
  ;[0.15 0.15 0.15 0.5] ResetValuesGameplayLoop
  (Variables|Default|SetLifes 3)
  (Variables|Default|SetFinishedIntroducing false)
  (Variables|Default|SetRoundPoints 0)
  (Variables|Default|SetPlayerLoaded false)
  (Variables|Default|SetGame%20Rule%20Selected -1))

(fn ConstructionScript)

(fn DefinePreferRule
  (params (NewRule :type Integer))
  (if (== (Variables|Default|GetGame%20Rule%20Selected) -1)
    (Variables|Default|SetGame%20Rule%20Selected NewRule)
    (Class|BPIGameplayLoop|GSPreferRuleSelected(Message) (Game|GetGameState) -1 (Variables|Default|GetGame%20Rule%20Selected))
    (return)
    (else
      (LocalVariables|SetL_OldRule (Variables|Default|GetGame%20Rule%20Selected))
      (bind _output_get (Variables|Default|SetGame%20Rule%20Selected NewRule))
      (Class|BPIGameplayLoop|GSPreferRuleSelected(Message) (Game|GetGameState) (LocalVariables|GetL_OldRule) _output_get)
      (return))))

(fn DefineEndGametime
  (params (GameDuration :type Integer)))

(fn HUDStartGameIntroducing
  (return 0))

(fn PSGetLifesRemaning
  (return (Variables|Default|GetLifes)))

(fn PSIsDead
  (return (<= (Variables|Default|GetLifes) 0)))