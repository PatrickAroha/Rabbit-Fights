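; Lobby game mode that seats joining players, tracks their network IDs and launches the match when everyone is ready.
; Each player gets a free PlayerStart from a slot array; logout frees it and tells all players to unready.
; Ready events check every BP_PlayerStateLobby, then server-travel to the Design map as listen host, passing IDs and player count in the URL.
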(event Custom|S_PlayersReady
  ;[0.15 0.15 0.15 0.5] Ready Config
  (CallFunction|CanStartGame))

(event Custom|S_StartGame
  ;[0.15 0.15 0.15 0.5] Start Game
  (for _array_element (Variables|Default|GetUnique%20Net%20Id)
    (if (Utilities|Enum|Equal(Enum) (Variables|Default|GetNetIDPlayers) "")
      (Variables|Default|SetNetIDPlayers (Class|AdvancedSessionsLibrary|UniqueNetIdtoString _array_element))
      (else
        (Variables|Default|SetNetIDPlayers (Utilities|String|Append (Variables|Default|GetNetIDPlayers) "," (Class|AdvancedSessionsLibrary|UniqueNetIdtoString _array_element)))
        (Variables|Default|SetPlayersLenght (Utilities|String|ToString(Integer) (Utilities|Array|Length (Variables|/Script/Engine.GameStateBase|GetPlayerArray (Game|GetGameState))))))))
  (Class|AdvancedSessionsLibrary|ServerTravel (Utilities|String|Append "Design?listen?IDs=" (Variables|Default|GetNetIDPlayers) "?NumPlayers=" (Variables|Default|GetPlayersLenght)) false false))

(event EventPostLogin
  (params (NewPlayer :type Player%20Controller%20Object%20Reference))
  ;[0.15 0.15 0.15 0.5] Login/Logout
  (Class|GameModeBase|RestartPlayer NewPlayer)
  (Utilities|Array|Add (Variables|Default|GetUnique%20Net%20Id) (Class|AdvancedSessionsLibrary|GetUniqueNetID NewPlayer)))

(event EventOnLogout
  (params (ExitingController :type Controller%20Object%20Reference))
  ;[0.15 0.15 0.15 0.5] Login/Logout
  (CallFunction|ClearSpawnSlot ExitingController)
  (CallFunction|ChangeAlltoNotReady***)
  (bind _asplayer_controller (Utilities|Casting|CastToPlayerController ExitingController))
  (Utilities|Array|RemoveItem (Variables|Default|GetUnique%20Net%20Id) (Class|AdvancedSessionsLibrary|GetUniqueNetID _asplayer_controller)))

(event EventPlayerReady
  ;[0.15 0.15 0.15 0.5] Ready Config
  (CallFunction|SPlayersReady))

(fn ConstructionScript)

(fn ChangeAlltoNotReady***
  (for _array_element (Variables|/Script/Engine.GameStateBase|GetPlayerArray (Game|GetGameState))
    (Class|BPILobby|GMChangeAlltoNotReady(Message) _array_element)))

(fn CanStartGame
  (for _array_element (Variables|/Script/Engine.GameStateBase|GetPlayerArray (Game|GetGameState))
    (bind _asbp_player_state_lobby (Utilities|Casting|CastToBP_PlayerStateLobby _array_element))
    (if (not (Default|GetReady _asbp_player_state_lobby))
      (LocalVariables|SetCanStart false)))
  (if (LocalVariables|GetCanStart)
    (CallFunction|SStartGame)))

(fn GetAllPlayerStartPoints
  (bind _outactors (Actor|GetAllActorsOfClass "/Script/Engine.PlayerStart"))
  (for _array_element _outactors
    (Utilities|Array|AddUnique (Variables|Default|GetPlayerStartPoints) (Utilities|Struct|MakeE_PlayerStartPoints _array_element 0 false))))

(fn ChoosePlayerStart
  (params (Player :type Controller%20Object%20Reference))
  (Utilities|IsValid (Utilities|Struct|BreakE_PlayerStartPoints (Utilities|Array|Get(acopy) (Variables|Default|GetPlayerStartPoints)))
    (:Is%20Valid
      _)
    (:Is%20Not%20Valid
      (CallFunction|GetAllPlayerStartPoints)))
  (for (_array_element _array_index) (Variables|Default|GetPlayerStartPoints)
    (if (not (.IsBusy (Utilities|Struct|BreakE_PlayerStartPoints _array_element)))
      (Utilities|Array|SetArrayElem (Variables|Default|GetPlayerStartPoints) _array_index (Utilities|Struct|MakeE_PlayerStartPoints (.PlayerStart (Utilities|Struct|BreakE_PlayerStartPoints _array_element)) Player true))
      (return (.PlayerStart (Utilities|Struct|BreakE_PlayerStartPoints _array_element))))))

(fn ClearSpawnSlot
  (params (InputPin :type Controller%20Object%20Reference))
  (for (_array_element _array_index) (Variables|Default|GetPlayerStartPoints)
    (if (== InputPin (.Controller (Utilities|Struct|BreakE_PlayerStartPoints _array_element)))
      (Utilities|Array|SetArrayElem (Variables|Default|GetPlayerStartPoints) _array_index (Utilities|Struct|MakeE_PlayerStartPoints (.PlayerStart (Utilities|Struct|BreakE_PlayerStartPoints _array_element)) 0 false)))))