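; Lobby game state that starts the game once the players in the lobby are ready.
; S_PlayersReady scans PlayerArray and checks the Ready flag on each BP_PlayerStateLobby.
; If none is unready, it triggers S_StartGame, which calls StartGame on BP_GameModeLobby.
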(event Custom|S_PlayersReady
  (Variables|Default|SetCanStartGame true)
  (for _array_element (Variables|Default|GetPlayerArray)
    (bind _asbp_player_state_lobby (Utilities|Casting|CastToBP_PlayerStateLobby _array_element))
    (if (not (Variables|/Game/Core/Lobby/BP_PlayerStateLobby.BP_PlayerStateLobby_C|GetReady _asbp_player_state_lobby))
      (Variables|Default|SetCanStartGame false)))
  (if (Variables|Default|GetCanStartGame)
    (CallFunction|SStartGame)))

(event Custom|S_StartGame
  (bind _asbp_game_mode_lobby (Utilities|Casting|CastToBP_GameModeLobby (Game|GetGameMode)))
  (Default|StartGame _asbp_game_mode_lobby))

(fn ConstructionScript)