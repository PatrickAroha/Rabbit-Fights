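; Lobby HUD Blueprint that picks which screen the local player sees on entering the lobby.
; CreateHudLobby waits briefly, then checks the given player state's unique net ID for session membership.
; Players in a session get a ready-button widget bound to their lobby player state and stored as the current layout.
; Anyone else gets the main menu widget.
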(event EventCreateHudLobby
  (params (PS :type Player%20State%20Object%20Reference))
  (Utilities|FlowControl|Delay 0.2)
  (bind _bisinsession (Class|AdvancedSessionsLibrary|IsPlayerinSession (Class|AdvancedSessionsLibrary|GetUniqueNetIDfromPlayerState PS)))
  (if _bisinsession
    (CallFunction|GenerateLobbyWidget PS)
    (else
      (CallFunction|GenerateMenuWidget))))

(fn ConstructionScript)

(fn GenerateLobbyWidget
  (params (Object :type Object%20Object%20Reference))
  (bind _asmy_player_state_lobby (Utilities|Casting|CastToMyPlayerStateLobby Object)
    (:then
      (bind _returnvalue (UserInterface|CreateWidget "/Game/Widgets/Lobby/W_LobbyReadyButton.W_LobbyReadyButton_C" (Game|Player|GetOwningPlayerController) _asmy_player_state_lobby))
      (bind _output_get (Variables|Default|SetWbCurrentLayout _returnvalue))
      (UserInterface|Viewport|AddtoViewport _output_get 0))
    (:CastFailed
      (Development|PrintString "Cast to MyPlayerStateLobby " true true "(R=1.000000,G=0.017391,B=0.000000,A=1.000000)" 1e+01))))

(fn GenerateMenuWidget
  (bind _returnvalue (UserInterface|CreateWidget "/Game/Widgets/Menu/W_menu.W_menu_C" (Game|Player|GetOwningPlayerController)))
  (UserInterface|Viewport|AddtoViewport _returnvalue 0))