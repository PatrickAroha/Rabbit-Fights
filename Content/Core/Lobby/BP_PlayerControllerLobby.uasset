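; Lobby player controller that shows the mouse cursor and switches the view between the player's pawn camera and the lobby camera.
; On possess, a short-delayed session check selects lobby mode for players in a session, or the pawn view otherwise.
; Creating a lobby also enters lobby mode, which triggers the pawn's ready-widget message and targets the level's CameraActor.
; A debug K key reopens the Lobby level and destroys the session.
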(event Custom|DefineViewToLobby
  ;[0.15 0.15 0.15 0.5] Lobby Setup
  (Utilities|FlowControl|DelayUntilNextTick)
  (bind _returnvalue (Actor|GetActorOfClass "/Script/Engine.CameraActor"))
  (Game|Player|SetViewTargetwithBlend _returnvalue 0.0 "VTBlend_Linear" 0.0 false))

(event Custom|RPC_PlayerStart
  (params (NewViewTarget :type Actor%20Object%20Reference))
  ;[1 0.266 0.266 0.5] OFF
)

(event Custom|DefineViewToPlayer
  (Utilities|FlowControl|DelayUntilNextTick)
  (bind _asbp_player_lobby (Utilities|Casting|CastToBP_PlayerLobby (Pawn|GetControlledPawn)))
  (Game|Player|SetViewTargetwithBlend (Components|GetOwner (Variables|/Game/Core/Lobby/BP_PlayerLobby.BP_PlayerLobby_C|GetCamera _asbp_player_lobby)) 0.0 "VTBlend_Linear" 0.0 false))

(event Custom|RS_ChangeToLobbyMode
  ;[0.15 0.15 0.15 0.5] Lobby Setup
  (Utilities|FlowControl|DelayUntilNextTick)
  (Class|BPILobby|PyActiveReadyWidget(Message) (Pawn|GetControlledPawn))
  (CallFunction|DefineViewtoLobby))

(event EventPossess
  (params (PossessedPawn :type Pawn%20Object%20Reference))
  (Utilities|FlowControl|Delay 0.2)
  (bind _bisinsession (Class|AdvancedSessionsLibrary|IsPlayerinSession (Class|AdvancedSessionsLibrary|GetUniqueNetIDfromPlayerState (Variables|/Script/Engine.Pawn|GetPlayerState PossessedPawn))))
  (if _bisinsession
    (CallFunction|RSChangetoLobbyMode)
    (else
      (CallFunction|DefineViewtoPlayer))))

(event EventPCPlayerCreateLobby
  ;[0.15 0.15 0.15 0.5] Lobby Setup
  (CallFunction|RSChangetoLobbyMode))

(event EventBeginPlay
  (Variables|Default|SetbShowMouseCursor true)
  (CallFunction|DefineViewtoPlayer))

(event Input|KeyboardEvents|K
  (params (Key :type Key%20Structure))
  ;[1 0.296 0.4072 0.5] DEBBUG DESCONECT
  (:Pressed
    (Game|OpenLevel(byName) "Lobby")
    (|DestroySession self)))

(fn ConstructionScript)