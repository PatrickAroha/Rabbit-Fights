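; BP_PlayerLobby is the lobby player actor that shows a player's ready state, Steam name and avatar through a 3D widget.
; Activation waits briefly, flags possession, binds to the lobby PlayerState's ready-update dispatcher and fetches the Steam nickname and avatar.
; RepNotify variables drive the display: possession creates the W_LobbyPlayerReady widget, while ready, name and avatar changes fire dispatchers.
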(event Custom|RS_ActivateWidget
  (Utilities|FlowControl|Delay 0.2)
  (Variables|Default|SetIsPossessed true)
  (bind _asbp_player_state_lobby (Utilities|Casting|CastToBP_PlayerStateLobby (Variables|Default|GetPlayerState)))
  (EventDispatchers|BindEventtoOnPSUpdateReady _asbp_player_state_lobby (EventDispatchers|CreateEvent :!event ChangedLobbyReady))
  (CallFunction|UpdateBind))

(event Custom|UpdateBind
  (bind _playerstate (Variables|Default|GetPlayerState))
  (bind _uniquenetid (Class|AdvancedSessionsLibrary|GetUniqueNetIDfromPlayerState _playerstate))
  (Variables|Default|SetSteamName (Utilities|Text|ToText(String) (Class|AdvancedIdentityLibrary|GetPlayerNickname _uniquenetid)))
  (bind _returnvalue (Class|AdvancedSteamFriendsLibrary|GetSteamFriendAvatar _uniquenetid "SteamAvatar_Medium")
    (:OnSuccess
      _)
    (:AsyncLoading
      _))
  (Variables|Default|SetSteamAvatar _returnvalue))

(event EventPyActiveReadyWidget
  (CallFunction|RSActivateWidget))

(event EventPUpdateAvatar
  (CallFunction|UpdateBind))

(fn ConstructionScript)

(fn Create3dWidgetReady
  (bind _returnvalue (UserInterface|CreateWidget "/Game/Widgets/Lobby/W_LobbyPlayerReady.W_LobbyPlayerReady_C" 0 0))
  (bind _output_get (Variables|Default|Set3DWidget _returnvalue))
  (UserInterface|SetWidget (Variables|Default|Get3dWidgetComponent) _output_get)
  (Class|BPILobby|Initialize(Message) (Variables|Default|Get3DWidget) self))

(fn OnRepIsPossessed
  (CallFunction|Create3dWidgetReady))

(fn OnRepLobbyReady
  (Default|CallChangedReadyState (Variables|Default|GetLobbyReady)))

(fn OnRepSteamName
  (Default|CallChangedSteamName (Variables|Default|GetSteamName)))

(fn OnRepSteamAvatar
  (Default|CallChangedSteamAvatar (Variables|Default|GetSteamAvatar)))

(fn ChangedLobbyReady
  (params (Ready :type Boolean))
  (Variables|Default|SetLobbyReady Ready))