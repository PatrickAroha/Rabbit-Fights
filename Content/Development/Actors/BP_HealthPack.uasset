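; Health pickup that heals overlapping Player-tagged actors through their Ability System Component.
; On overlap it compares two attribute reads and, only if they differ, applies a fixed heal and consumes the pack.
; Consumption disables collision and hides the mesh through the Visible OnRep, then a delay makes it collectable again.
; A timeline for bobbing and spinning the mesh exists but is never run.
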(event OnComponentBeginOverlap(PackCollision)
  (params (OverlappedComponent :type Primitive%20Component%20Object%20Reference) (OtherActor :type Actor%20Object%20Reference) (OtherComp :type Primitive%20Component%20Object%20Reference) (OtherBodyIndex :type Integer) (bFromSweep :type Boolean) (SweepResult :type Hit%20Result%20Structure%20%28by%20ref%29))
  (bind _returnvalue (Ability|GetAbilitySystemComponent OtherActor))
  (if (Actor|ActorHasTag OtherActor "Player")
    (Utilities|IsValid _returnvalue
      (:Is%20Valid
        (CallFunction|Overlap _returnvalue)))))

(event Custom|DefinePackNotColletable
  (Variables|Default|SetVisible false)
  (Collision|SetCollisionEnabled (Variables|Default|GetPackCollision) "NoCollision")
  (Utilities|FlowControl|Delay 25.0)
  (CallFunction|DefinePackColletable))

(event Custom|DefinePackColletable
  (Variables|Default|SetVisible true)
  (Collision|SetCollisionEnabled (Variables|Default|GetPackCollision) "QueryOnly"))

(event Custom|Overlap
  (params (ASC :type Ability%20System%20Component%20Object%20Reference))
  (if (not (== (.ReturnValue (Ability|Attribute|GetFloatAttributefromAbilitySystemComponent ASC "(AttributeName=\"Health\",Attribute=/Script/Deep.BasicAttributeSet:Health,AttributeOwner=\"/Script/CoreUObject.Class'/Script/Deep.BasicAttributeSet'\")")) (.ReturnValue (Ability|Attribute|GetFloatAttributefromAbilitySystemComponent ASC "(AttributeName=\"MaxHealth\",Attribute=/Script/Deep.BasicAttributeSet:MaxHealth,AttributeOwner=\"/Script/CoreUObject.Class'/Script/Deep.BasicAttributeSet'\")"))))
    (CallFunction|PlayerHealMagnitude ASC 0 0 3e+01)
    (CallFunction|DefinePackNotColletable)))

(fn ConstructionScript)

(fn ExposePack)

(fn OnRepVisible
  (Rendering|SetVisibility (Variables|Default|GetHealthPack) (Variables|Default|GetVisible) false))