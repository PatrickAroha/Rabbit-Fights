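; Item spawner actor that, shortly after BeginPlay, drops one BP_PickUp holding a randomly chosen item from ItensToSpawn.
; TrySpawnItem picks a random navigable point within the Sphere radius, raises it to a random height, and capsule-traces downward, retrying without limit until it hits a "Floor"-tagged component.
; The trace leaves persistent debug drawing.
; CalculatePlayerSpawnLocation computes a random in-bounds point but is not called here.
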(event Custom|SpawnItem
  (bind _spawnlocation (CallFunction|TrySpawnItem))
  (bind _returnvalue (Game|SpawnActorfromClass "/Game/Development/Systems/Inventory/BP_PickUp.BP_PickUp_C" (Math|Transform|MakeTransform _spawnlocation "0, 0, 0" "1.000000,1.000000,1.000000") "Undefined" "MultiplyWithRoot" 0 0))
  (bind _returnvalue_2 (Game|ConstructObjectfromClass (.OutItem (Utilities|Array|Random (Variables|Default|GetItensToSpawn)))))
  (Variables|/Script/Deep.PickUp|SetItem _returnvalue _returnvalue_2)
  (Default|Init _returnvalue))

(event EventBeginPlay
  (Utilities|FlowControl|Delay 0.2)
  (CallFunction|SpawnItem))

(fn ConstructionScript)

(fn TrySpawnItem
  (bind _sphere (Variables|Default|GetSphere))
  (bind _randomlocation (Class|NavigationSystemV1|GetRandomLocationinNavigableRadius (Transformation|GetWorldLocation (Variables|Default|GetSphere)) (Components|Sphere|GetScaledSphereRadius _sphere) 0 0 :!label _label))
  (bind _output_get (LocalVariables|SetLocationToSpawn (Math|Vector|MakeVector (.X (Math|Vector|BreakVector _randomlocation)) (.Y (Math|Vector|BreakVector _randomlocation)) (+ (.Z (Math|Vector|BreakVector (Transformation|GetWorldLocation _sphere))) (Math|Random|RandomFloatinRange 4e+02 5.5e+02) 48.0))))
  (bind _outhit (Collision|CapsuleTraceByChannel _output_get (- _output_get "0.000000,0.000000,3000.000000") 8e+01 8e+01 "TraceTypeQuery1" true 0 "Persistent"))
  (if (Components|ComponentHasTag (.HitComponent (Collision|BreakHitResult _outhit)) "Floor")
    (return (LocalVariables|GetLocationToSpawn))
    (else
      (goto _label))))

(fn CalculatePlayerSpawnLocation
  (bind _sphere (Variables|Default|GetSphere))
  (bind _returnvalue (Transformation|GetWorldLocation _sphere))
  (bind _returnvalue_2 (Components|Sphere|GetScaledSphereRadius _sphere))
  (bind _returnvalue_3 (Math|Random|RandomPointinBoundingBox _returnvalue (Math|Vector|MakeVector _returnvalue_2 _returnvalue_2 _returnvalue_2)))
  (return (Math|Vector|MakeVector (.x _returnvalue_3) (.y _returnvalue_3) (Math|Float|Max(Float) (.Z (Math|Vector|BreakVector _returnvalue)) (.z _returnvalue_3)))))