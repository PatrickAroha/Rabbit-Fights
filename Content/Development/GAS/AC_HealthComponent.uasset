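; Actor component that handles a player's death for the health system.
; Die forwards to PlayerDie, which notifies the owner pawn's PlayerState of the death and sends a die message with killer and weapon to the owner.
; With a valid killer pawn, it sends the game mode a kill round-point message for that killer's BP_PlayerState and updates its kill count.
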(event Custom|PlayerDie
  (params (Killer :type Actor%20Object%20Reference) (Weapon :type Actor%20Object%20Reference))
  (bind _aspawn (Utilities|Casting|CastToPawn (Components|GetOwner)))
  (Class|BPIGameplayLoop|PSUpdateDeaths(Message) (Variables|/Script/Engine.Pawn|GetPlayerState _aspawn))
  (Class|BPIHealth|CDie(Message) (Components|GetOwner) Killer Weapon)
  (Utilities|IsValid Killer
    (:Is%20Valid
      (bind _aspawn_2 (Utilities|Casting|CastToPawn Killer))
      (bind _asbp_player_state (Utilities|Casting|CastToBP_PlayerState (Variables|/Script/Engine.Pawn|GetPlayerState _aspawn_2)))
      (Class|BPIGameplayLoop|GMRoundPoint(Message) (Game|GetGameMode) _asbp_player_state "(TagName=\"RoundPoint.Kill\")")
      (Default|UpdateKillValue _asbp_player_state))))

(event EventDie
  (params (Killer :type Actor%20Object%20Reference) (Weapon :type Actor%20Object%20Reference))
  (CallFunction|PlayerDie Killer Weapon))