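; Gameplay ability for a ground-targeted magic AOE attack that damages pawns around a confirmed location.
; A looping targeting montage plays while a ground-trace decal target actor awaits user confirmation.
; Confirming commits the ability, shows an indicator cue and plays the throw montage until the ThunderBolt event arrives.
; That event triggers an authority-only sphere trace, applying SetByCaller instant damage once per actor, excluding the caster, and removes the cue.
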(event Custom|LoopTargetingAnimation
  ;[0.15 0.15 0.15 0.5] TargetingPhase
  (|PlayMontageandWaitProxy "None" "/Game/PlayerAsset/Animations2/Montages/M_TargetingMagic.M_TargetingMagic" 1.0 "None" true 1.0 0.0 false
    (:OnBlendOut
      (if (Variables|Default|GetIsWaitingTargetData)
        (CallFunction|LoopTargetingAnimation)))
    (:OnInterrupted
      (if (Variables|Default|GetIsWaitingTargetData)
        (Ability|EndAbility)))))

(event Custom|ConfirmStrike
  ;[0.15 0.15 0.15 0.5] AttackPhase
  (bind _returnvalue (Ability|CommitAbility))
  (if _returnvalue
    (Class|GameplayAbility|AddGameplayCuewithParams "(TagName=\"GameplayCue.AEOIndicator\")" (Ability|GameplayCue|MakeGameplayCueParameters :RawMagnitude (* (Variables|Default|GetMagnitude) 2.0) :Location (Variables|Default|GetConfirmedAOELocation)) true)
    (|PlayMontageandWaitProxy "None" "/Game/PlayerAsset/Animations2/Montages/M_ThrowMagic.M_ThrowMagic" 1.0 "None" true 1.0 0.0 false
      (:then
        (Ability|Tasks|WaitGameplayEvent "(TagName=\"Event.Magics.Shoot.ThunderBolt\")" 0
          (:EventReceived
            (CallFunction|AOEDamage)
            (GameplayCue|RemoveGameplayCue "(TagName=\"GameplayCue.AEOIndicator\")"))))
      (:OnCompleted
        (Ability|EndAbility :!label _label))
      (:OnInterrupted
        (goto _label)))
    (else
      (Ability|EndAbility))))

(event Custom|AOEDamage
  (bind _confirmedaoelocation (Variables|Default|GetConfirmedAOELocation))
  ;[0.15 0.15 0.15 0.5] AttackPhase
  (Ability|HasAuthority
    (:True
      (bind _outhits (Collision|MultiSphereTraceForObjects _confirmedaoelocation _confirmedaoelocation (Variables|Default|GetAOERadius) (Utilities|Array|MakeArray "ObjectTypeQuery3") false (Utilities|Array|MakeArray (Ability|GetAvatarActorfromActorInfo)) "ForDuration"))
      (Utilities|Array|Clear (Variables|Default|GetHitsActors))
      (for _array_element _outhits
        (if (not (Utilities|Array|ContainsItem (Variables|Default|GetHitsActors) (.HitActor (Collision|BreakHitResult _array_element))))
          (Utilities|Array|AddUnique (Variables|Default|GetHitsActors) (.HitActor (Collision|BreakHitResult _array_element)))
          (Utilities|IsValid (Ability|GetAbilitySystemComponent (.HitActor (Collision|BreakHitResult _array_element)))
            (:Is%20Valid
              (bind _returnvalue (Ability|GameplayEffect|AssignTagSetbyCallerMagnitude (Ability|MakeOutgoingGameplayEffectSpec "/Game/Development/GAS/Effects/GE_DamageInstant.GE_DamageInstant_C") "(TagName=\"Data.Damage\")" (Variables|Default|GetMagnitude)))
              (GameplayEffects|ApplyGameplayEffectSpecToSelf (Ability|GetAbilitySystemComponent (.HitActor (Collision|BreakHitResult _array_element))) _returnvalue))))))))

(event Ability|EventActivateAbility
  ;[0.15 0.15 0.15 0.5] TargetingPhase
  (CallFunction|LoopTargetingAnimation)
  (Variables|Default|SetIsWaitingTargetData true)
  (bind _data (|WaitTargetData :ConfirmationType "UserConfirmed" :Class "/Game/Development/GAS/TargetingActors/GA_TargetActor_GroundTrace_Decal.GA_TargetActor_GroundTrace_Decal_C" :Decal%20Size (* (Variables|Default|GetAOERadius) 2.0) :Decal 0 :MaxRange 1.3e+03 :StartLocation (Class|GameplayAbility|MakeTargetLocationInfofromOwnerActor) :ReticleClass 0 :bDebug true)
    (:ValidData
      (Variables|Default|SetIsWaitingTargetData false)
      (Variables|Default|SetConfirmedAOELocation (.Location (Collision|BreakHitResult (Ability|TargetData|GetHitResultfromTargetData _data))))
      (CallFunction|ConfirmStrike))))