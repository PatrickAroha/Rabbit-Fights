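; Gameplay ability that casts the Charm spell, spawning a BP_Charm actor toward the traced aim point.
; On activation it turns the avatar to the camera's forward direction, ignores move input until the ability ends, clears the Charm cue and plays a shoot montage.
; The montage's Shoot event commits cooldown and runs an instant line trace, whose end point feeds the authority-only spawn from a socket.
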(event Ability|EventActivateAbility
  (bind _rot (Class|BPIPlayer|CamGetForwarDirection(Message) (Ability|GetAvatarActorfromActorInfo)))
  (Transformation|SetActorRotation (Ability|GetAvatarActorfromActorInfo) _rot)
  (Input|SetIgnoreMoveInput (Game|GetPlayerController (Variables|/Script/Engine.Pawn|GetPlayerState (.AsPawn (Utilities|Casting|CastToPawn (Ability|GetAvatarActorfromActorInfo))))) true)
  (GameplayCue|RemoveGameplayCue "(TagName=\"GameplayCue.Magics.Charm\")")
  (|PlayMontageandWaitProxy "None" "/Game/PlayerAsset/Animations2/Montages/AM_ShootMagicAnimation_Montage.AM_ShootMagicAnimation_Montage" 1.0 "None" true 1.0 0.0 true
    (:then
      (Ability|Tasks|WaitGameplayEvent "(TagName=\"Event.Magics.Shoot\")" 0
        (:EventReceived
          (Ability|CommitAbilityCooldown false)
          (bind _data (|WaitTargetData :ConfirmationType "Instant" :Class "/Script/GameplayAbilities.GameplayAbilityTargetActor_SingleLineTrace" :MaxRange 999.0 :TraceProfile "(Name=\"NoCollision\")" :StartLocation (Class|GameplayAbility|MakeTargetLocationInfofromOwnerActor) :ReticleClass 0 :bDebug true)
            (:ValidData
              (bind _location (Class|BPIPlayer|GAGetSocketLocation(Message) (Ability|GetAvatarActorfromActorInfo) "NewEnumerator0"))
              (|SpawnActor 0 _location "0, 0, 0" "/Game/Development/Systems/Magics/Charm/BP_Charm.BP_Charm_C" true (Class|AbilitySystemBlueprintLibrary|GetTargetDataEndPoint _data) (.AsPawn (Utilities|Casting|CastToPawn (Ability|GetAvatarActorfromActorInfo)))
                (:Success
                  (Ability|EndAbility))))))))
    (:OnCompleted
      (Ability|EndAbility :!label _label))
    (:OnInterrupted
      (goto _label))
    (:OnCancelled
      (goto _label))))

(event Ability|EventOnEndAbility
  (params (bWasCancelled :type Boolean))
  (Input|SetIgnoreMoveInput (Game|GetPlayerController (Variables|/Script/Engine.Pawn|GetPlayerState (.AsPawn (Utilities|Casting|CastToPawn (Ability|GetAvatarActorfromActorInfo))))) false))