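; GA_EquipWeapon is an event-triggered gameplay ability that swaps the avatar's equipped weapon.
; After committing, it finds the avatar's ItemManager component and switches on the first target tag in the event data.
; The wand and mace tags equip their matching weapon Blueprints, and any other tag unequips the weapon.
; The ability then ends, though only when a valid ItemManager was found.
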(event Ability|EventActivateAbilityFromEvent
  (params (EventData :type Gameplay%20Event%20Data%20Structure%20%28by%20ref%29))
  (bind _returnvalue (Ability|GetAvatarActorfromActorInfo))
  (bind _returnvalue_2 (Actor|GetComponentbyClass _returnvalue "/Game/Weapons/ItemManager.ItemManager_C"))
  (Ability|CommitAbility)
  (Utilities|IsValid _returnvalue_2
    (:Is%20Valid
      (Utilities|FlowControl|Sequence
        (:then_0
          (|SwitchGameplayTag (Utilities|Array|Get(acopy) (GameplayTags|BreakGameplayTagContainer (Utilities|Struct|BreakGameplayEventData EventData)))
            (:Default
              (Default|UnequipWeapon _returnvalue_2))
            (:Weapon.Ranged.Wand
              (Default|EquipItem _returnvalue_2 "/Game/Weapons/BP_Weapon_Wand.BP_Weapon_Wand_C"))
            (:Weapon.Melee.Mace
              (Default|EquipItem _returnvalue_2 "/Game/Weapons/BP_Weapon_Mace.BP_Weapon_Mace_C"))))
        (:then_1
          (Ability|EndAbility))))))