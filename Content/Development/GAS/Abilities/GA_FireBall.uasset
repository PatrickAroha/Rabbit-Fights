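; Gameplay ability that casts a fireball from the avatar toward a targeted point.
; It plays a shooting montage, waits for the Event.Magics.Shoot gameplay event, then requests instant target data.
; It removes the fireball cue and spawns BP_FireBall on authority above an interface-supplied socket location, passing the target end point.
; Spawn success or montage completion, interruption or cancellation ends the ability, and cooldown is committed only on end.
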(event Ability|EventActivateAbility
  (bind _returnvalue (Class|GameplayAbility|MakeTargetLocationInfofromOwnerActor))
  (|PlayMontageandWaitProxy "None" "/Game/PlayerAsset/Animations2/Montages/AM_ShootMagicAnimation_Montage.AM_ShootMagicAnimation_Montage" 1.0 "None" true 1.0 0.0 true
    (:then
      (Ability|Tasks|WaitGameplayEvent "(TagName=\"Event.Magics.Shoot\")" 0
        (:EventReceived
          (bind _data (|WaitTargetData :ConfirmationType "Instant" :Class "/Script/GameplayAbilities.GameplayAbilityTargetActor_SingleLineTrace" :MaxRange 9999.0 :TraceProfile "(Name=\"Trace\")" :StartLocation (Utilities|Struct|MakeGameplayAbilityTargetingLocationInfo (.sourceactor _returnvalue) (.sourcecomponent _returnvalue) (.sourceability _returnvalue) (Math|Transform|MakeTransform (+ (.location (.literaltransform _returnvalue)) "0.000000,0.000000,50.000000") (.rotation (.literaltransform _returnvalue)) (.scale (.literaltransform _returnvalue))) (.sourcesocketname _returnvalue) (.locationtype _returnvalue)) :ReticleClass "")
            (:ValidData
              (bind _location (Class|BPIPlayer|GAGetSocketLocation(Message) (Ability|GetAvatarActorfromActorInfo) "NewEnumerator0"))
              (GameplayCue|RemoveGameplayCue "(TagName=\"GameplayCue.Magics.FireBall\")")
              (|SpawnActor 0 (+ _location "0.000000,0.000000,50.000000") "0, 0, 0" "/Game/Development/Systems/Magics/Fireball/BP_FireBall.BP_FireBall_C" true (Class|AbilitySystemBlueprintLibrary|GetTargetDataEndPoint _data) (.AsPawn (Utilities|Casting|CastToPawn (Ability|GetAvatarActorfromActorInfo)))
                (:Success
                  (Ability|EndAbility))))))))
    (:OnCompleted
      (Ability|EndAbility :!label _label))
    (:OnInterrupted
      (goto _label))
    (:OnCancelled
      (goto _label))))

(event Ability|EventOnEndAbility
  (params (bWasCancelled :type Boolean))
  (Ability|CommitAbilityCooldown false))