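; Gameplay ability for the MaceBoink melee attack, but its attack logic is disconnected from activation.
; Activation only looks up the avatar's ItemManager and ends if it is missing.
; The unreachable chain plays the attack montage and, on authority, uses HitScan gameplay events to start and stop weapon hit scanning with a set-by-caller instant damage spec.
; Ending the ability stops hit scanning on any valid weapon.
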(event Ability|EventActivateAbility
  (Utilities|IsValid (Actor|GetComponentbyClass (Ability|GetAvatarActorfromActorInfo) "/Game/Weapons/ItemManager.ItemManager_C")
    (:Is%20Not%20Valid
      (Ability|EndAbility))))

(event Ability|EventOnEndAbility
  (params (bWasCancelled :type Boolean))
  (bind _equipedweapon (Variables|Default|GetEquipedWeapon)
    (:then
      (Default|HitScanEnd _equipedweapon))
    (:else)))