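; Gameplay ability that casts a magic shield on the avatar, replacing the fireball cue.
; It plays a cast montage with a spawn cue and locks move input until the shoot event arrives.
; That event applies the shield effect, adds its cue and restores movement.
; A shield-break event removes effect and cue and ends the ability; cooldown is committed on ability end.
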(event Ability|EventActivateAbility
  (bind _returnvalue (Ability|GetAvatarActorfromActorInfo))
  (bind _aspawn (Utilities|Casting|CastToPawn _returnvalue))
  (bind _playerstate (Variables|/Script/Engine.Pawn|GetPlayerState _aspawn))
  (bind _returnvalue_2 (Game|GetPlayerController _playerstate))
  (GameplayCue|RemoveGameplayCue "(TagName=\"GameplayCue.Magics.FireBall\")")
  (|PlayMontageandWaitProxy "None" "/Game/PlayerAsset/Animations2/mAGICS/M_Shild.M_Shild" 1.0 "None" true 1.0 0.0 true
    (:then
      (Ability|Tasks|WaitGameplayEvent "(TagName=\"Event.Magics.Shoot\")" 0 true
        (:then
          (Ability|Tasks|WaitGameplayEvent "(TagName=\"Event.ActivateAbility.ShieldBreak\")" 0
            (:then
              (Input|SetIgnoreMoveInput _returnvalue_2 true)
              (GameplayCue|AddGameplayCue :GameplayCueTag "(TagName=\"GameplayCue.SpawnShild\")"))
            (:EventReceived
              (GameplayCue|RemoveGameplayCue "(TagName=\"GameplayCue.Magics.Shild\")")
              (Ability|RemoveGameplayEffectFromOwnerWithHandle (Variables|Default|GetShildSpec))
              (Ability|EndAbility))))
        (:EventReceived
          (bind _returnvalue_3 (Ability|ApplyGameplayEffectToOwner "/Game/Development/GAS/Effects/GE_Shild.GE_Shild_C"))
          (Variables|Default|SetShildSpec _returnvalue_3)
          (Class|GameplayAbility|AddGameplayCuewithParams "(TagName=\"GameplayCue.Magics.Shild\")" (Ability|GameplayCue|MakeGameplayCueParameters :Instigator _aspawn) false)
          (Input|SetIgnoreMoveInput _returnvalue_2 false))))))

(event Ability|EventOnEndAbility
  (params (bWasCancelled :type Boolean))
  (Ability|CommitAbilityCooldown false))