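; Gameplay ability for a Giant potion that temporarily raises the avatar's max health and heals it, alongside a gameplay cue removed on ability end.
; Activation applies set-by-caller max-health and instant-heal effects, all keyed on Data.Heal, then ends after a short fixed delay.
; On end, it sets max health to a hardcoded 100 and, if the queried attribute is found, redefines health capped at that value.
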(event Ability|EventActivateAbility
  (GameplayCue|AddGameplayCue :GameplayCueTag "(TagName=\"GameplayCue.Potions.Giant\")")
  (bind _returnvalue (Spec|MakeSpecHandle(ByClass) "/Game/Development/GAS/Effects/GE_DefineMaxHealth.GE_DefineMaxHealth_C" 0))
  (bind _returnvalue_2 (Ability|GameplayEffect|AssignTagSetbyCallerMagnitude _returnvalue "(TagName=\"Data.Heal\")" 4e+02))
  (GameplayEffects|ApplyGameplayEffectSpecToSelf (Ability|GetAbilitySystemComponent (Ability|GetAvatarActorfromActorInfo)) _returnvalue_2)
  (bind _returnvalue_3 (Spec|MakeSpecHandle(ByClass) "/Game/Development/GAS/Effects/GE_HealInstant.GE_HealInstant_C" 0))
  (bind _returnvalue_4 (Ability|GameplayEffect|AssignTagSetbyCallerMagnitude _returnvalue_3 "(TagName=\"Data.Heal\")" 3e+02))
  (GameplayEffects|ApplyGameplayEffectSpecToSelf (Ability|GetAbilitySystemComponent (Ability|GetAvatarActorfromActorInfo)) _returnvalue_4)
  (Ability|Tasks|WaitDelay 2.0
    (:OnFinish
      (Ability|EndAbility))))

(event Ability|EventOnEndAbility
  (params (bWasCancelled :type Boolean))
  (bind _returnvalue (Ability|GetAvatarActorfromActorInfo))
  (bind _returnvalue_2 (Ability|GetAbilitySystemComponent _returnvalue))
  (bind (_bfound _returnvalue_3) (Class|AbilitySystemComponent|GetGameplayAttributeValue _returnvalue_2 "(AttributeName=\"Health\",Attribute=/Script/Deep.BasicAttributeSet:Health,AttributeOwner=\"/Script/CoreUObject.Class'/Script/Deep.BasicAttributeSet'\")"))
  (bind _returnvalue_4 (Spec|MakeSpecHandle(ByClass) "/Game/Development/GAS/Effects/GE_DefineMaxHealth.GE_DefineMaxHealth_C" 0))
  (bind _returnvalue_5 (Ability|GameplayEffect|AssignTagSetbyCallerMagnitude _returnvalue_4 "(TagName=\"Data.Heal\")" 1e+02))
  (GameplayEffects|ApplyGameplayEffectSpecToSelf _returnvalue_2 _returnvalue_5)
  (if _bfound
    (bind _returnvalue_6 (Spec|MakeSpecHandle(ByClass) "/Game/Development/GAS/Effects/GE_DefineHealth.GE_DefineHealth_C" 0))
    (bind _returnvalue_7 (Ability|GameplayEffect|AssignTagSetbyCallerMagnitude _returnvalue_6 "(TagName=\"Data.Heal\")" (Math|Float|SelectFloat 1e+02 _returnvalue_3 (> _returnvalue_3 1e+02))))
    (GameplayEffects|ApplyGameplayEffectSpecToSelf (Ability|GetAbilitySystemComponent (Ability|GetAvatarActorfromActorInfo)) _returnvalue_7)))