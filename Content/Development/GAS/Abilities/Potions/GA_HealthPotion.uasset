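; Gameplay ability for a health potion that heals the player by a fixed amount when activated.
; On activation it checks for authority, passes the avatar's Ability System Component to PlayerHealMagnitude, then ends the ability.
; The non-authority branch does nothing, so both the heal and the EndAbility call run only with authority.
; The LocationToSpawn graph holds only unused transform nodes.
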(event Ability|EventActivateAbility
  (Ability|HasAuthority
    (:True
      (CallFunction|PlayerHealMagnitude (Ability|GetAbilitySystemComponent (Ability|GetAvatarActorfromActorInfo)) 0 0 3e+01)
      (Ability|EndAbility))))

(event Ability|EventOnEndAbility
  (params (bWasCancelled :type Boolean)))