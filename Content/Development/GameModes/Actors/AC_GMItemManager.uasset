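; AC_GMItemManager is a game mode item manager component that extends a parent item manager on player pawns.
; Equipping caches the owner's BP_PlayerState and sets the item's carrier before calling the parent logic; unequipping defers to the parent.
; Round points go to the game mode with that player state and the item's point type tag.
; Owner death is forwarded to the carried item as a message with killer and victim.
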(event EventRoundPoint
  (Class|BPIGameplayLoop|GMRoundPoint(Message) (Game|GetGameMode) (Variables|Default|GetAs%20BP%20Player%20State) (Variables|/Script/Deep.GMItem|GetRoundPointType (Variables|Default|GetItem))))

(event EventUnequipItem
  (params (Killer :type Actor%20Object%20Reference))
  (|CallParentFunction Killer))

(event EventPlayerOwnerDie
  (params (Killer :type Actor%20Object%20Reference) (Victim :type Actor%20Object%20Reference))
  (Class|BPIPlayerDied|PlayerOwnerDie(Message) (Variables|Default|GetCarriedItem) Killer Victim))

(event EventEquipItem
  (params (NewItem :type GM%20Item%20Object%20Reference) (NewCarriedItem :type Actor%20Object%20Reference))
  (bind _aspawn (Utilities|Casting|CastToPawn (Components|GetOwner)))
  (bind _asbp_player_state (Utilities|Casting|CastToBP_PlayerState (Variables|/Script/Engine.Pawn|GetPlayerState _aspawn)))
  (Variables|Default|SetAs%20BP%20Player%20State _asbp_player_state)
  (Variables|/Script/Deep.GMItem|SetCarrier NewItem (Components|GetOwner))
  (|CallParentFunction NewItem NewCarriedItem))