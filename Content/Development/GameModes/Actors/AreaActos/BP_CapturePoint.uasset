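; Game-mode capture point that marks a lone player inside its sphere as holder by equipping an item through their GMItemManager component.
; On the server, each overlap begin or end clears the current holder and re-evaluates, so a contested zone has no holder.
; OwnerDie also clears the holder and offers the role to the killer if exactly one player overlaps the sphere.
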(event OnComponentBeginOverlap(Sphere)
  (params (OverlappedComponent :type Primitive%20Component%20Object%20Reference) (OtherActor :type Actor%20Object%20Reference) (OtherComp :type Primitive%20Component%20Object%20Reference) (OtherBodyIndex :type Integer) (bFromSweep :type Boolean) (SweepResult :type Hit%20Result%20Structure%20%28by%20ref%29))
  (Networking|SwitchHasAuthority
    (:Authority
      (CallFunction|RemovePlayerPointer)
      (CallFunction|ChangePlayers OtherActor))))

(event OnComponentEndOverlap(Sphere)
  (params (OverlappedComponent :type Primitive%20Component%20Object%20Reference) (OtherActor :type Actor%20Object%20Reference) (OtherComp :type Primitive%20Component%20Object%20Reference) (OtherBodyIndex :type Integer))
  (bind _sphere (Variables|Default|GetSphere))
  (bind _overlappingactors (Collision|GetOverlappingActors _sphere "/Game/Core/BP_Player.BP_Player_C" :!class /Script/Engine.PrimitiveComponent))
  (bind _output (Utilities|Array|Get(acopy) _overlappingactors))
  (Networking|SwitchHasAuthority
    (:Authority
      (CallFunction|RemovePlayerPointer)
      (Utilities|IsValid _output
        (:Is%20Valid
          (CallFunction|ChangePlayers _output))))))

(event Custom|RemovePlayerPointer
  (Utilities|IsValid (Variables|Default|GetPlayerPointer)
    (:Is%20Valid
      (Utilities|IsValid (Actor|GetComponentbyClass (Variables|Default|GetPlayerPointer) "/Script/Deep.GMItemManager")
        (:Is%20Valid
          (Class|GMItemManager|RSUnequipItem (Actor|GetComponentbyClass (Variables|Default|GetPlayerPointer) "/Script/Deep.GMItemManager"))
          (Variables|Default|SetPlayerPointer 0))))))

(event Custom|ChangePlayers
  (params (Target :type Actor%20Object%20Reference))
  (if (Actor|ActorHasTag Target "Player")
    (if (== (Utilities|Array|Length (Collision|GetOverlappingActors (Variables|Default|GetSphere) "/Game/Core/BP_Player.BP_Player_C" :!class /Script/Engine.PrimitiveComponent)) 1)
      (CallFunction|NewPlayerPointer Target)
      (else
        (CallFunction|RemovePlayerPointer)))))

(event Custom|NewPlayerPointer
  (params (Player :type Actor%20Object%20Reference))
  (bind _ascharacter (Utilities|Casting|CastToCharacter Player))
  (bind _output_get (Variables|Default|SetPlayerPointer _ascharacter))
  (Class|GMItemManager|RSEquipItem (Actor|GetComponentbyClass _output_get "/Script/Deep.GMItemManager") (Variables|Default|GetItem) self))

(event EventOwnerDie
  (params (Killer :type Actor%20Object%20Reference))
  (Networking|SwitchHasAuthority
    (:Authority
      (CallFunction|RemovePlayerPointer)
      (CallFunction|ChangePlayers Killer))))

(fn ConstructionScript)