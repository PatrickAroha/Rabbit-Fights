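; Area actor that keeps a fixed population of ten magic sword pickups on the ground inside its sphere.
; BeginPlay fills the count, and SwordMagicCollected decrements it and spawns a replacement.
; Each location comes from a random navigable point, capsule-traced downward from above and retried without limit until it hits a Floor-tagged component.
; Spawned BP_MagicSwordGround actors receive this actor as their Spawner.
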(event Custom|SpawnLocation
  (bind _locationtospawna (CallFunction|TrySpawnPlayer))
  (Game|SpawnActorfromClass "/Game/Development/GameModes/Actors/ItensActors/BP_MagicSwordGround.BP_MagicSwordGround_C" (Math|Transform|MakeTransform _locationtospawna "0, 0, 0" "1.000000,1.000000,1.000000") "Undefined" "MultiplyWithRoot" 0 self 0))

(event EventBeginPlay
  (CallFunction|SpawnCounter))

(event EventSwordMagicCollected
  (Math|Integer|DecrementInt (Variables|Default|GetSwordsCounts)
    (:%20%20
      (CallFunction|SpawnCounter))))

(fn ConstructionScript
  (|CallParentFunction))

(fn TrySpawnPlayer
  (bind _sphere (Variables|Default|GetSphere))
  (bind _randomlocation (Class|NavigationSystemV1|GetRandomLocationinNavigableRadius (Transformation|GetWorldLocation _sphere) (Components|Sphere|GetScaledSphereRadius _sphere) 0 0 :!label _label))
  (bind _outhit (Collision|CapsuleTraceByChannel (Math|Vector|MakeVector (.X (Math|Vector|BreakVector _randomlocation)) (.Y (Math|Vector|BreakVector _randomlocation)) (+ (.Z (Math|Vector|BreakVector (Transformation|GetWorldLocation _sphere))) (Math|Random|RandomFloatinRange 4e+02 5.5e+02) 48.0)) (- (Math|Vector|MakeVector (.X (Math|Vector|BreakVector _randomlocation)) (.Y (Math|Vector|BreakVector _randomlocation)) (+ (.Z (Math|Vector|BreakVector (Transformation|GetWorldLocation _sphere))) (Math|Random|RandomFloatinRange 4e+02 5.5e+02) 48.0)) "0.000000,0.000000,3000.000000") 8e+01 8e+01 "TraceTypeQuery1" false 0 "None" true "(R=1.000000,G=0.000000,B=0.000000,A=1.000000)" "(R=0.000000,G=1.000000,B=0.000000,A=1.000000)" 0.0))
  (if (Components|ComponentHasTag (.HitComponent (Collision|BreakHitResult _outhit)) "Floor")
    (return (- (.Location (Collision|BreakHitResult _outhit)) "0.000000,0.000000,50.000000"))
    (else
      (goto _label))))

(fn SpawnCounter
  (while (< (Variables|Default|GetSwordsCounts) 10)
    (CallFunction|SpawnLocation)
    (Math|Integer|IncrementInt (Variables|Default|GetSwordsCounts)))
  (return))