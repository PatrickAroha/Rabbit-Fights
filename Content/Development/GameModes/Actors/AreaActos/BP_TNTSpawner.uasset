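; Server-driven spawner that drops BP_TNT at random spots inside a movable, resizable sphere.
; A looping timer handles spawning, and authority Tick periodically restarts it with a shorter delay until it reaches a minimum.
; Spawn points are random navigable locations raised above the sphere, retried until a downward capsule trace hits a "Floor"-tagged component.
; After four TNT actors exist, it reuses pooled invisible ones, which return through TNTUpdateStatus.
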(event Custom|SpawnTNT
  (if (< (+ (Utilities|Array|Length (Variables|Default|GetSpawnedsActors)) (Utilities|Array|Length (Variables|Default|GetInvTNTActors))) 4)
    (bind _spawnlocation (CallFunction|TrySpawnItem))
    (bind _returnvalue (Game|SpawnActorfromClass "/Game/Development/GameModes/Actors/ItensActors/BP_TNT.BP_TNT_C" (Math|Transform|MakeTransform _spawnlocation "0, 0, 0" "1.000000,1.000000,1.000000") "Undefined" "MultiplyWithRoot" 0 self 0))
    (Utilities|Array|Add (Variables|Default|GetSpawnedsActors) _returnvalue)
    (else
      (CallFunction|SpawnInvisibleTNT))))

(event Custom|UpdateSpawnerLocation
  (params (NewLocation :type Vector) (InSphereRadius :type Float%20%28single-precision%29))
  (Utilities|FlowControl|DelayUntilNextTick)
  (Transformation|SetWorldLocation (Variables|Default|GetSphere) NewLocation false true)
  (Components|Sphere|SetSphereRadius (Variables|Default|GetSphere) InSphereRadius false))

(event Custom|Timer
  (params (InputPin :type Float%20%28double-precision%29))
  (Networking|SwitchHasAuthority
    (:Authority
      (if (>= (Variables|Default|GetMinSpawnInterval) (Variables|Default|GetTimerToInitSpawn))
        (Actor|Tick|SetActorTickEnabled false)
        (else
          (CallFunction|StartSpawner InputPin))))))

(event Custom|InitSpawnTnt
  (Networking|SwitchHasAuthority
    (:Authority
      (bind _returnvalue (Utilities|Time|SetTimerbyEvent (EventDispatchers|CreateEvent :!event Custom|SpawnTNT) (Variables|Default|GetTimerToInitSpawn) true))
      (Variables|Default|SetHandleSpawnTNT _returnvalue))))

(event EventTick
  (params (DeltaSeconds :type Float%20%28single-precision%29))
  (CallFunction|Timer DeltaSeconds))

(event EventBeginPlay
  (CallFunction|InitSpawnTnt))

(event EventTNTUpdateStatus
  (params (TNT :type Actor%20Object%20Reference))
  (CallFunction|UpdateTntStatus TNT))

(fn ConstructionScript
  (|CallParentFunction))

(fn TrySpawnItem
  (bind _sphere (Variables|Default|GetSphere))
  (bind _randomlocation (Class|NavigationSystemV1|GetRandomLocationinNavigableRadius (Transformation|GetWorldLocation _sphere) (Components|Sphere|GetScaledSphereRadius _sphere) 0 0 :!label _label))
  (bind _output_get (Variables|Default|SetLocationToSpawn (Math|Vector|MakeVector (.X (Math|Vector|BreakVector _randomlocation)) (.Y (Math|Vector|BreakVector _randomlocation)) (+ (.Z (Math|Vector|BreakVector (Transformation|GetWorldLocation _sphere))) (Math|Random|RandomFloatinRange 4e+02 5.5e+02) 48.0))))
  (bind _outhit (Collision|CapsuleTraceByChannel _output_get (- _output_get "0.000000,0.000000,3000.000000") 8e+01 8e+01 "TraceTypeQuery1" false 0 "None" true "(R=1.000000,G=0.000000,B=0.000000,A=1.000000)" "(R=0.000000,G=1.000000,B=0.000000,A=1.000000)" 0.0))
  (if (Components|ComponentHasTag (.HitComponent (Collision|BreakHitResult _outhit)) "Floor")
    (return (Variables|Default|GetLocationToSpawn))
    (else
      (goto _label))))

(fn StartSpawner
  (params (Tick :type Float%20%28double-precision%29))
  (bind _output_get (Variables|Default|SetCurrentTime (+ Tick (Variables|Default|GetCurrentTime))))
  (if (>= _output_get (Variables|Default|GetInterval))
    (CallFunction|DefineNewInterval)
    (else
      (return))))

(fn DefineNewInterval
  (Utilities|Time|ClearandInvalidateTimerbyHandle (Variables|Default|GetHandleSpawnTNT))
  (Variables|Default|SetCurrentTime 0.0)
  (Variables|Default|SetTimerToInitSpawn (Math|Float|Clamp(Float) (- (Variables|Default|GetTimerToInitSpawn) 0.1) (Variables|Default|GetMinSpawnInterval) 5.0))
  (CallFunction|InitSpawnTnt))

(fn SpawnInvisibleTNT
  (bind _spawnlocation (CallFunction|TrySpawnItem))
  (bind _output_get (LocalVariables|SetSelectedTnt (.OutItem (Utilities|Array|Random (Variables|Default|GetInvTNTActors)))))
  (Class|BPIActors|TNTDefineLocationtoSpawn(Message) _output_get _spawnlocation)
  (Utilities|Array|RemoveItem (Variables|Default|GetInvTNTActors) (LocalVariables|GetSelectedTnt))
  (Utilities|Array|Add (Variables|Default|GetSpawnedsActors) (LocalVariables|GetSelectedTnt)))

(fn UpdateTntStatus
  (params (NewItem :type Actor%20Object%20Reference%20%28by%20ref%29))
  (Utilities|Array|RemoveItem (Variables|Default|GetSpawnedsActors) NewItem)
  (Utilities|Array|Add (Variables|Default|GetInvTNTActors) NewItem))