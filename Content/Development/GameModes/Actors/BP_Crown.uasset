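; BP_Crown is a game mode crown pickup that is worn by whoever takes it and passes to the killer when its owner dies.
; On server overlap, it disables sphere collision, equips its item through the actor's GMItemManager and attaches itself to the character mesh's Crown socket.
; OwnerDie detaches the crown, then repeats the item equip and socket attach on the Killer.
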(event OnComponentBeginOverlap(Sphere)
  (params (OverlappedComponent :type Primitive%20Component%20Object%20Reference) (OtherActor :type Actor%20Object%20Reference) (OtherComp :type Primitive%20Component%20Object%20Reference) (OtherBodyIndex :type Integer) (bFromSweep :type Boolean) (SweepResult :type Hit%20Result%20Structure%20%28by%20ref%29))
  (Networking|SwitchHasAuthority
    (:Authority
      (Collision|SetCollisionEnabled (Variables|Default|GetSphere) "NoCollision")
      (Class|GMItemManager|RSEquipItem (Actor|GetComponentbyClass OtherActor "/Script/Deep.GMItemManager") (Variables|Default|GetItem) self)
      (CallFunction|EquipCrown OtherActor))))

(event Custom|EquipCrown
  (params (Target :type Actor%20Object%20Reference))
  (Utilities|IsValid Target
    (:Is%20Valid
      (bind _ascharacter (Utilities|Casting|CastToCharacter Target))
      (Utilities|IsValid _ascharacter
        (:Is%20Valid
          (Utilities|IsValid (Variables|/Script/Engine.Character|GetMesh _ascharacter)
            (:Is%20Valid
              (Transformation|AttachComponentToComponent self (Variables|/Script/Engine.Character|GetMesh _ascharacter) "Crown" "SnapToTarget" "SnapToTarget" "KeepWorld" true))))))))

(event EventOwnerDie
  (params (Killer :type Actor%20Object%20Reference))
  (Transformation|DetachFromActor "KeepWorld" "KeepWorld" "KeepWorld")
  (Class|GMItemManager|RSEquipItem (Actor|GetComponentbyClass Killer "/Script/Deep.GMItemManager") (Variables|Default|GetItem) self)
  (CallFunction|EquipCrown Killer))

(fn ConstructionScript)