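; Ground pickup actor for the magic sword, collected when a player interacts with it.
; Interact builds a single full-durability magic sword item from its data asset and offers it to the player's inventory.
; Without checking the pickup result, it then hides the sphere hierarchy and disables sphere and mesh collision.
; After a short delay it notifies its spawner that the sword was collected and destroys itself.
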(event EventInteract
  (params (Player :type Pawn%20Object%20Reference))
  (bind _returnvalue (Game|ConstructObjectfromClass "/Game/Development/Systems/Inventory/Itens/MagicSword/Item_MagicSword.Item_MagicSword_C"))
  (Variables|/Script/Deep.ItemInstance|SetQuantity _returnvalue 1)
  (Variables|/Script/Deep.ItemInstance|SetDef _returnvalue "/Game/Development/Systems/Inventory/Itens/MagicSword/DA_MagicSword.DA_MagicSword")
  (Variables|/Script/Deep.ItemInstance|SetDurability _returnvalue 1.0)
  (Class|InventoryComponent|TryPickUpItem (CallFunction|GetInventory Player) _returnvalue)
  (Rendering|SetVisibility (Variables|Default|GetSphere) false true)
  (Collision|SetCollisionEnabled (Variables|Default|GetSphere) "NoCollision")
  (Utilities|FlowControl|Delay 1.5)
  (Class|BPIActors|SwordMagicCollected(Message) (Variables|Default|GetSpawner))
  (Actor|DestroyActor))

(fn ConstructionScript
  (|CallParentFunction))