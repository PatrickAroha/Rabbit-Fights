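; TNT actor that drops to the ground, bounces up and explodes, damaging nearby players.
; A downward trace sets the landing point, and two chained timelines animate the spinning fall and the rise, triggered on BeginPlay or when a spawn location is set.
; The blast hides the mesh, notifies TntSpawner, and sphere-overlaps BP_Player pawns.
; Radial damage is applied through a GAS instant effect using set-by-caller magnitude.
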(event Custom|Explosion
  (bind _returnvalue (Transformation|GetActorLocation))
  (bind _mesh_tnt (Variables|Default|GetMesh_TNT))
  (Transformation|SetWorldRotation (Variables|Default|GetMesh_TNT) "0, 0, 0" false false)
  (bind (_outhit _returnvalue_2) (Collision|LineTraceByChannel _returnvalue (- _returnvalue "0.000000,0.000000,1000.000000") "TraceTypeQuery1" false 0 "None"))
  (if _returnvalue_2
    (bind _movement (Timeline|Downthrowble PlayFromStart)
      (:Update
        (Transformation|SetWorldLocation _mesh_tnt (Math|Vector|Lerp(Vector) (Transformation|GetActorLocation) (- (.Location (Collision|BreakHitResult _outhit)) "0.000000,0.000000,-40.000000") _movement) false false)
        (Transformation|SetWorldRotation _mesh_tnt (Math|Rotator|Lerp(Rotator) "0, 0, 0" "0.000000,0.000000,-470.000000" _movement) false false))
      (:Finished
        (Variables|Default|SetWorldLocation (Transformation|GetWorldLocation (Variables|Default|GetMesh_TNT)))
        (Components|Timeline|PlayfromStart (Variables|Default|GetForwardThrowble))))))

(event Custom|SetLocation
  (params (InputPin :type Vector))
  (Rendering|SetVisibility (Variables|Default|GetMesh_TNT) true false)
  (Transformation|SetWorldLocation (Variables|Default|GetMesh_TNT) InputPin false false)
  (CallFunction|Explosion))

(event EventTNTDefineLocationtoSpawn
  (params (LocationToSpawn :type Vector :default "0, 0, 0"))
  (CallFunction|SetLocation LocationToSpawn))

(event EventBeginPlay
  (CallFunction|Explosion))

(fn ConstructionScript)

(fn CalculateDamage
  (params (InputPin :type Ability%20System%20Component%20Object%20Reference) (InputPin2 :type Float%20%28double-precision%29))
  (bind _returnvalue (Spec|MakeSpecHandle(ByClass) "/Game/Development/GAS/Effects/GE_DamageInstant.GE_DamageInstant_C" 0 self))
  (bind _returnvalue_2 (Ability|GameplayEffect|AssignTagSetbyCallerMagnitude _returnvalue "(TagName=\"Data.Damage\")" InputPin2))
  (GameplayEffects|ApplyGameplayEffectSpecToSelf InputPin _returnvalue_2))