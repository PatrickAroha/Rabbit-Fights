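; BP_CollectTissue is a point-type actor for a game mode that awards a round point when the killer collects enough tissues.
; On each killer tissue capture, it compares the collected count to the GameState PlayerArray size and calls the parent's MakeRoudPoint once the count reaches it.
; Equipping runs no logic, while unequipping clears the round-point timer if the player state is valid.
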(event EventMakeRoudPoint
  (|CallParentFunction))

(event EventOnEquipped)

(event EventOnUnequipped
  (params (KillerActor :type Actor%20Object%20Reference))
  (bind _bp_player_state (Variables|Default|GetBP%20Player%20State))
  (Utilities|IsValid _bp_player_state
    (:Is%20Valid
      (Utilities|Time|ClearandInvalidateTimerbyHandle _bp_player_state (Variables|Default|GetMakeRoundPointTimer)))))

(event EventOnKillerCaputeTissue
  (params (QtyCollectedsTissue :type Integer))
  (if (>= QtyCollectedsTissue (Utilities|Array|Length (Variables|/Script/Engine.GameStateBase|GetPlayerArray (Game|GetGameState (Variables|Default|GetBP%20Player%20State)))))
    (Class|GMItem|MakeRoudPoint)))