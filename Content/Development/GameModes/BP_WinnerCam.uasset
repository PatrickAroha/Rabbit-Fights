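; BP_WinnerCam is a spring-arm camera actor that, judging by its name, frames the match winner with a short intro move.
; On becoming the view target it caches its rotation and location, then plays the Zoom timeline from the start.
; The timeline's single track is meant to drive three lerps together: shortening the spring arm, swinging the yaw and lowering the actor from its cached transform.
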(event EventOnBecomeViewTarget
  (params (PC :type Player%20Controller%20Object%20Reference))
  (Variables|Default|SetRotation (Transformation|GetActorRotation))
  (Variables|Default|SetLocation (Transformation|GetActorLocation))
  (Components|Timeline|PlayfromStart (Variables|Default|GetZoom)))

(fn ConstructionScript)