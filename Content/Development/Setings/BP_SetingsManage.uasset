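; BP_SetingsManage provides helper functions that apply the game's display and audio settings.
; Resolution and screen mode functions map an index to 720p or 1080p and to fullscreen or windowed on GameUserSettings, without calling apply or save.
; The volume function overrides a given sound class's volume within a supplied sound mix, then pushes that mix so the change takes effect.
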(fn SetResolution
  (params (index :type Integer))
  (bind _returnvalue (Settings|GetGameUserSettings))
  (switch int index
    (:0
      (Class|GameUserSettings|SetScreenResolution _returnvalue (Utilities|Struct|MakeIntPoint 1280 720)))
    (:1
      (Class|GameUserSettings|SetScreenResolution _returnvalue (Utilities|Struct|MakeIntPoint 1920 1080)))))

(fn SetScreenSize
  (params (index :type Integer))
  (bind _returnvalue (Settings|GetGameUserSettings))
  (switch int index
    (:0
      (Class|GameUserSettings|SetFullscreenMode _returnvalue "Fullscreen"))
    (:1
      (Class|GameUserSettings|SetFullscreenMode _returnvalue "Windowed"))))

(fn SetSoundVolumes
  (params (Value :type Float%20%28double-precision%29) (WorldContextObject :type Object%20Object%20Reference) (InSoundClass :type Sound%20Class%20Object%20Reference) (InSoundMixModifier :type Sound%20Mix%20Object%20Reference))
  (Audio|SetSoundMixClassOverride WorldContextObject InSoundMixModifier InSoundClass Value 1.0 1.0 true)
  (Audio|PushSoundMixModifier WorldContextObject InSoundMixModifier))