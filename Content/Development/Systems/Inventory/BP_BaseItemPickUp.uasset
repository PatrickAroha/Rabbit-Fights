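; BP_BaseItemPickUp is a base pickup for the inventory system that represents a collectible item in the world.
; The construction script sets its static mesh from the ActorMesh of the item held in its Item variable.
; Item replicates with a RepNotify that reapplies the mesh when both the item and its mesh are valid.
; CollectItem reports whether the item is valid and returns it, without removing the pickup itself.
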(fn ConstructionScript
  (bind _item (Variables|Default|GetItem))
  (Utilities|IsValid (.item _item)
    (:Is%20Valid
      (Components|StaticMesh|SetStaticMesh (Variables|Default|GetStaticMesh) (Variables|/Game/Development/Systems/Inventory/PDA_DefineItemInfo.PDA_DefineItemInfo_C|GetActorMesh (.item _item))))))

(fn OnRepItem
  (bind _item (Variables|Default|GetItem))
  (bind _actormesh (Variables|/Game/Development/Systems/Inventory/PDA_DefineItemInfo.PDA_DefineItemInfo_C|GetActorMesh (.item _item)))
  (Utilities|IsValid (.item _item)
    (:Is%20Valid
      (Utilities|IsValid _actormesh
        (:Is%20Valid
          (Components|StaticMesh|SetStaticMesh (Variables|Default|GetStaticMesh) _actormesh))))))

(fn CollectItem
  (Utilities|IsValid (.item (Variables|Default|GetItem))
    (:Is%20Valid
      (return true (Variables|Default|GetItem)))
    (:Is%20Not%20Valid
      (return false ""))))