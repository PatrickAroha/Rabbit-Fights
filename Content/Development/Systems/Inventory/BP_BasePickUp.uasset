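; BP_BasePickUp is a base pickup Blueprint in the inventory system that displays the mesh of the item it holds.
; The construction script validates Item and its Def, then applies the definition's mesh to MeshComp.
; BeginPlay does nothing, and a disconnected copy of the mesh assignment in the event graph never runs.
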(event EventBeginPlay)

(fn ConstructionScript
  (bind _item (Variables|Default|GetItem))
  (bind _def (Variables|/Script/Deep.ItemInstance|GetDef _item))
  (Utilities|IsValid _item
    (:Is%20Valid
      (Utilities|IsValid _def
        (:Is%20Valid
          (Components|StaticMesh|SetStaticMesh (Variables|Default|GetMeshComp) (Variables|/Script/Deep.ItemDefinition|GetMesh _def)))))))