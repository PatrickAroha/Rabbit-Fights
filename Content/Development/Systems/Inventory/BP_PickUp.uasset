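; Inventory pickup actor that displays an item in the world through a static mesh and particle system.
; After a short delay on BeginPlay, Init applies the item definition's mesh and Cascade effect, then an empty Destroy event is called.
; When destroyed, it sends an item-collected message to the SpawnerManager.
; A randomly timed self-destruct and a construction-script copy of the visual setup are left disconnected.
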(event Custom|Init
  (bind _item (Variables|Default|GetItem))
  (bind _def (Variables|/Script/Deep.ItemInstance|GetDef _item))
  (bind _itemmesh (Variables|/Script/Deep.ItemDefinition|GetItemMesh _def))
  (bind _cascadeeffect (Variables|/Script/Deep.ItemDefinition|GetCascadeEffect _def))
  (Utilities|IsValid _item
    (:Is%20Valid
      (Utilities|IsValid _def
        (:Is%20Valid
          (Utilities|IsValid _cascadeeffect
            (:Is%20Valid
              (Effects|Components|ParticleSystem|SetTemplate (Variables|Default|GetParticleSystem) _cascadeeffect))
            (:Is%20Not%20Valid
              _))
          (Utilities|IsValid _itemmesh
            (:Is%20Valid
              (Components|StaticMesh|SetStaticMesh (Variables|Default|GetStaticMesh) _itemmesh))))))))

(event Custom|Destroy)

(event EventBeginPlay
  (Utilities|FlowControl|Delay 0.2)
  (CallFunction|Init)
  (CallFunction|Destroy))

(event EventDestroyed
  (Class|BPIGameplayEvents|ItemCollected(Message) (Variables|Default|GetSpawnerManager)))

(fn ConstructionScript)