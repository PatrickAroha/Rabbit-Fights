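; BP_BaseProjectile is a base projectile that flies toward a target location and deals damage through the Gameplay Ability System.
; On BeginPlay it aims ProjectileMovement at TargetLocation, scaled by Speed, and activates it.
; A sphere overlap with a non-instigator actor owning an ability system component applies the DamageType effect with Magnitude as SetByCaller Data.Damage, then destroys the projectile.
; Any sphere hit also destroys it.
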(event OnComponentBeginOverlap(Sphere)
  (params (OverlappedComponent :type Primitive%20Component%20Object%20Reference) (OtherActor :type Actor%20Object%20Reference) (OtherComp :type Primitive%20Component%20Object%20Reference) (OtherBodyIndex :type Integer) (bFromSweep :type Boolean) (SweepResult :type Hit%20Result%20Structure%20%28by%20ref%29))
  (bind _returnvalue (Ability|GetAbilitySystemComponent OtherActor))
  (bind _self self)
  (if (!= OtherActor (Variables|Actor|GetInstigator))
    (Utilities|IsValid OtherActor
      (:Is%20Valid
        (Utilities|IsValid _returnvalue
          (:Is%20Valid
            (bind _returnvalue_2 (Spec|MakeSpecHandle(ByClass) (Variables|Default|GetDamageType) _self _self))
            (bind _returnvalue_3 (Ability|GameplayEffect|AssignTagSetbyCallerMagnitude _returnvalue_2 "(TagName=\"Data.Damage\")" (Variables|ProjectileSettings|GetMagnitude)))
            (GameplayEffects|ApplyGameplayEffectSpecToSelf _returnvalue _returnvalue_3)
            (Actor|DestroyActor)))))))

(event OnComponentHit(Sphere)
  (params (HitComponent :type Primitive%20Component%20Object%20Reference) (OtherActor :type Actor%20Object%20Reference) (OtherComp :type Primitive%20Component%20Object%20Reference) (NormalImpulse :type Vector :default "0, 0, 0") (Hit :type Hit%20Result%20Structure%20%28by%20ref%29))
  (Actor|DestroyActor))

(event EventBeginPlay
  (bind _projectilemovement (Variables|Default|GetProjectileMovement))
  (Variables|/Script/Engine.MovementComponent|SetVelocity _projectilemovement (* (Math|Vector|GetUnitDirection(Vector) (Transformation|GetActorLocation) (Variables|ProjectileSettings|GetTargetLocation)) (Variables|ProjectileSettings|GetSpeed)))
  (Components|Activation|Activate _projectilemovement false))

(fn ConstructionScript)