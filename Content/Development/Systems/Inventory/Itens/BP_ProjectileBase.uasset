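; Base projectile that, on the server, flies toward a target location and expires after a set duration.
; Overlapping a non-instigator Player-tagged actor with an Ability System Component triggers cleanup and passes both to the empty OnOverlap hook.
; Component hits only forward to the empty OnHit hook, without ending the projectile.
; Cleanup hides the body, disables its collision and shows the VFX briefly before destroying the actor.
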(event OnComponentBeginOverlap(PlayerOverlap1)
  (params (OverlappedComponent :type Primitive%20Component%20Object%20Reference) (OtherActor :type Actor%20Object%20Reference) (OtherComp :type Primitive%20Component%20Object%20Reference) (OtherBodyIndex :type Integer) (bFromSweep :type Boolean) (SweepResult :type Hit%20Result%20Structure%20%28by%20ref%29))
  (bind _returnvalue (Ability|GetAbilitySystemComponent OtherActor))
  (if (and (!= (Variables|Actor|GetInstigator) OtherActor) (Actor|ActorHasTag OtherActor "Player"))
    (Utilities|IsValid OtherActor
      (:Is%20Valid
        (Utilities|IsValid _returnvalue
          (:Is%20Valid
            (CallFunction|Hidden)
            (CallFunction|Overlap OtherActor _returnvalue)))))))

(event OnComponentHit(PlayerOverlap)
  (params (HitComponent :type Primitive%20Component%20Object%20Reference) (OtherActor :type Actor%20Object%20Reference) (OtherComp :type Primitive%20Component%20Object%20Reference) (NormalImpulse :type Vector :default "0, 0, 0") (Hit :type Hit%20Result%20Structure%20%28by%20ref%29))
  (CallFunction|Hit OtherActor))

(event Custom|Hidden
  (Rendering|SetVisibility (Variables|Default|GetPlayerOverlap) false true)
  (Collision|SetCollisionEnabled (Variables|Default|GetPlayerOverlap) "NoCollision")
  (Rendering|SetVisibility (Variables|Default|GetProjectileVFX) true false)
  (Utilities|FlowControl|Delay (Variables|BaseValues|GetDurationVFXs))
  (Rendering|SetVisibility (Variables|Default|GetProjectileVFX) false false)
  (Components|DestroyComponent (Variables|Default|GetProjectileVFX))
  (Actor|DestroyActor))

(event Custom|Overlap
  (params (Actor :type Actor%20Object%20Reference) (AbilitySystem :type Ability%20System%20Component%20Object%20Reference))
  (CallFunction|OnOverlap Actor))

(event Custom|Hit
  (params (Actor :type Actor%20Object%20Reference))
  (CallFunction|OnHit Actor))

(event EventBeginPlay
  (Networking|SwitchHasAuthority
    (:Authority
      (Variables|/Script/Engine.MovementComponent|SetVelocity (Variables|Default|GetProjectileMovement) (* (Math|Vector|GetUnitDirection(Vector) (Transformation|GetActorLocation) (Variables|BaseValues|GetTargetLocation)) (Variables|BaseValues|GetSpeed)))
      (Components|Activation|Activate (Variables|Default|GetProjectileMovement) false)
      (Utilities|FlowControl|Delay (Variables|BaseValues|GetDuration))
      (CallFunction|Hidden))))

(fn ConstructionScript)

(fn OnOverlap
  (params (Actor :type Actor%20Object%20Reference)))

(fn OnHit
  (params (Actor :type Actor%20Object%20Reference)))