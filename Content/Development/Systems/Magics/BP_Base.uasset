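; Base Blueprint for magic actors that supplies shared explosion, damage and hit-detection helpers, and calls Hidden three seconds after BeginPlay.
; Effect plays the explosion particle and sound at PlayerOverlap, while DebbugExplosionRange sphere-queries nearby BP_Player pawns there.
; CalculateDamage applies GE_DamageInstant through GAS with a SetByCaller Data.Damage magnitude.
; Hit and overlap events defer to the parent, and RadialDamageCalculate holds only an unused distance-falloff expression.
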(event Custom|Effect
  (Effects|SpawnEmitteratLocation "/Game/Art/VFX/FXVarietyPack/Particles/P_ky_explosion.P_ky_explosion" (Transformation|GetWorldLocation (Variables|Default|GetPlayerOverlap)) "0, 0, 0" "0.800000,0.800000,0.800000")
  (Audio|PlaySoundatLocation "/Engine/VREditor/Sounds/UI/Flashlight_Switch.Flashlight_Switch" (Transformation|GetWorldLocation (Variables|Default|GetPlayerOverlap)) "0, 0, 0" 1.0 1.0 0.0 0 0 0 0))

(event EventBeginPlay
  (|CallParentFunction)
  (Utilities|FlowControl|Delay 3.0)
  (CallFunction|Hidden))

(fn ConstructionScript
  (|CallParentFunction))

(fn CalculateDamage
  (params (AC :type Ability%20System%20Component%20Object%20Reference) (Damage :type Float%20%28double-precision%29))
  (bind _returnvalue (Spec|MakeSpecHandle(ByClass) "/Game/Development/GAS/Effects/GE_DamageInstant.GE_DamageInstant_C" (Game|GetInstigator) self))
  (bind _returnvalue_2 (Ability|GameplayEffect|AssignTagSetbyCallerMagnitude _returnvalue "(TagName=\"Data.Damage\")" Damage))
  (GameplayEffects|ApplyGameplayEffectSpecToSelf AC _returnvalue_2))

(fn OnHit
  (params (Actor :type Actor%20Object%20Reference))
  (|CallParentFunction Actor))

(fn OnOverlap
  (params (Actor :type Actor%20Object%20Reference))
  (|CallParentFunction Actor))