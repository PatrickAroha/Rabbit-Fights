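; BP_MagicPickUp is a magic item pickup that takes its visible mesh from its assigned MagicItem.
; The construction script sets MeshComp to the item's PickupMesh when both the item and mesh are valid.
; An Init event applies the same mesh again, checking only that MagicItem is valid.
; The graphs shown contain only this visual setup, with no collection logic.
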(event Custom|Init
  (bind _magicitem (Variables|Default|GetMagicItem))
  (Utilities|IsValid _magicitem
    (:Is%20Valid
      (Components|StaticMesh|SetStaticMesh (Variables|Default|GetMeshComp) (Variables|/Script/Deep.MagicItemDefinition|GetPickupMesh _magicitem)))))

(fn ConstructionScript
  (bind _magicitem (Variables|Default|GetMagicItem))
  (bind _pickupmesh (Variables|/Script/Deep.MagicItemDefinition|GetPickupMesh _magicitem))
  (Utilities|IsValid _magicitem
    (:Is%20Valid
      (Utilities|IsValid _pickupmesh
        (:Is%20Valid
          (Components|StaticMesh|SetStaticMesh (Variables|Default|GetMeshComp) _pickupmesh))))))