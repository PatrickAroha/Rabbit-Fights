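; BP_Charm is a magic projectile that charms the actor it overlaps.
; On overlap it plays an explosion and sound, passes its instigator to the target, activates GA_Charmed on the target's ability system and hides.
; Hits just hide it; both paths fast-forward the projectile VFX by whatever remains of two seconds since spawn.
; Damage and radius helpers exist but are not called here.
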(event Custom|Teste)

(event Custom|Effect
  (Effects|SpawnEmitteratLocation "/Game/Art/VFX/FXVarietyPack/Particles/P_ky_explosion.P_ky_explosion" (Transformation|GetWorldLocation (Variables|Default|GetPlayerOverlap)) "0, 0, 0" "0.800000,0.800000,0.800000")
  (Audio|PlaySoundatLocation "/Engine/VREditor/Sounds/UI/Flashlight_Switch.Flashlight_Switch" (Transformation|GetWorldLocation (Variables|Default|GetPlayerOverlap)) "0, 0, 0" 1.0 1.0 0.0 0 0 0 0))

(event Custom|PowerAbility
  (params (Enemy :type Actor%20Object%20Reference))
  (bind _returnvalue (Ability|GetAbilitySystemComponent Enemy))
  (Utilities|IsValid _returnvalue
    (:Is%20Valid
      (Class|BPIPlayerGAS|SetCharmedInstigator(Message) Enemy (Game|GetInstigator))
      (Abilities|TryActivateAbilitybyClass _returnvalue "/Game/Development/GAS/Abilities/GA_Charmed.GA_Charmed_C" true)
      (CallFunction|Hidden))))

(event EventBeginPlay
  (|CallParentFunction)
  (Variables|Default|SetStartTime (Utilities|Time|GetGameTimeinSeconds)))

(fn ConstructionScript
  (|CallParentFunction))

(fn CalculateDamage
  (params (AC :type Ability%20System%20Component%20Object%20Reference) (Damage :type Float%20%28double-precision%29))
  (bind _returnvalue (Spec|MakeSpecHandle(ByClass) "/Game/Development/GAS/Effects/GE_DamageInstant.GE_DamageInstant_C" (Game|GetInstigator) self))
  (bind _returnvalue_2 (Ability|GameplayEffect|AssignTagSetbyCallerMagnitude _returnvalue "(TagName=\"Data.Damage\")" Damage))
  (GameplayEffects|ApplyGameplayEffectSpecToSelf AC _returnvalue_2))

(fn SGE
  (params (ASC :type Ability%20System%20Component%20Object%20Reference)))

(fn OnHit
  (params (Actor :type Actor%20Object%20Reference))
  (|CallParentFunction Actor)
  (CallFunction|Hidden)
  (Class|NiagaraComponent|AdvanceSimulationbyTime (Variables|Default|GetProjectileVFX) (Math|Float|Max(Float) (- 2.0 (- (Utilities|Time|GetGameTimeinSeconds) (Variables|Default|GetStartTime))) 0.0) (Utilities|Time|GetWorldDeltaSeconds)))

(fn OnOverlap
  (params (Actor :type Actor%20Object%20Reference))
  (|CallParentFunction Actor)
  (CallFunction|Effect)
  (CallFunction|PowerAbility Actor)
  (Class|NiagaraComponent|AdvanceSimulationbyTime (Variables|Default|GetProjectileVFX) (Math|Float|Max(Float) (- 2.0 (- (Utilities|Time|GetGameTimeinSeconds) (Variables|Default|GetStartTime))) 0.0) (Utilities|Time|GetWorldDeltaSeconds)))