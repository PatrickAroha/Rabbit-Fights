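; UperDash explosive magic projectile that damages players through the Gameplay Ability System and removes itself after a short lifetime.
; Overlapping a player other than the instigator deals flat damage, while a blocking hit damages nearby players using RadialDamageCalculate.
; Both paths play explosion effects, then hide and destroy the actor.
; CalculateDamage applies GE_DamageInstant, passing the amount as a SetByCaller Data.Damage magnitude.
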(event OnComponentHit(Sphere)
  (params (HitComponent :type Primitive%20Component%20Object%20Reference) (OtherActor :type Actor%20Object%20Reference) (OtherComp :type Primitive%20Component%20Object%20Reference) (NormalImpulse :type Vector :default "0, 0, 0") (Hit :type Hit%20Result%20Structure%20%28by%20ref%29))
  (CallFunction|Hit))

(event OnComponentBeginOverlap(Sphere)
  (params (OverlappedComponent :type Primitive%20Component%20Object%20Reference) (OtherActor :type Actor%20Object%20Reference) (OtherComp :type Primitive%20Component%20Object%20Reference) (OtherBodyIndex :type Integer) (bFromSweep :type Boolean) (SweepResult :type Hit%20Result%20Structure%20%28by%20ref%29))
  (CallFunction|Overlap OtherActor))

(event Custom|Hit
  (CallFunction|Effect)
  (CallFunction|Damage))

(event Custom|Effect
  (Effects|SpawnEmitteratLocation "/Game/Art/VFX/FXVarietyPack/Particles/P_ky_explosion.P_ky_explosion" (Transformation|GetWorldLocation (Variables|Default|GetSphere)) "0, 0, 0" "0.800000,0.800000,0.800000")
  (Audio|PlaySoundatLocation "/Engine/VREditor/Sounds/UI/Flashlight_Switch.Flashlight_Switch" (Transformation|GetWorldLocation (Variables|Default|GetSphere)) "0, 0, 0" 1.0 1.0 0.0 0 0 0 0))

(event Custom|Damage
  (bind _outputpin (Utilities|DebbugExplosionRange))
  (for _array_element _outputpin
    (Utilities|IsValid (Ability|GetAbilitySystemComponent _array_element)
      (:Is%20Valid
        (CallFunction|CalculateDamage (Ability|GetAbilitySystemComponent _array_element) (Utilities|RadialDamageCalculate _array_element)))))
  (CallFunction|Hidden))

(event Custom|Hidden
  (bind _sphere (Variables|Default|GetSphere))
  (Rendering|SetVisibility _sphere false true)
  (Collision|SetCollisionEnabled _sphere "NoCollision")
  (Utilities|FlowControl|Delay 0.2)
  (Components|DestroyComponent (Variables|Default|GetProjectileVFX))
  (Actor|DestroyActor))

(event Custom|Overlap
  (params (Actor :type Actor%20Object%20Reference))
  (if (and (!= Actor (Variables|Default|GetInstigator)) (Actor|ActorHasTag Actor "Player"))
    (CallFunction|CalculateDamage (Ability|GetAbilitySystemComponent Actor) 1e+01)
    (CallFunction|Effect)
    (CallFunction|Hidden)))

(event Custom|CustomEvent
  (Utilities|Time|SetTimerbyEvent (delegate Custom|CustomEvent_0) 0.0))

(event Custom|CustomEvent_0
  (Actor|DestroyActor))

(event EventBeginPlay
  (|CallParentFunction)
  (Utilities|FlowControl|Delay 3.0)
  (CallFunction|Hidden))

(fn ConstructionScript
  (|CallParentFunction))

(fn CalculateDamage
  (params (AC :type Ability%20System%20Component%20Object%20Reference) (Damage :type Float%20%28double-precision%29))
  (bind _returnvalue (Spec|MakeSpecHandle(ByClass) "/Game/Development/GAS/Effects/GE_DamageInstant.GE_DamageInstant_C" (Game|GetInstigator) self))
  (bind _returnvalue_2 (Ability|GameplayEffect|AssignTagSetbyCallerMagnitude _returnvalue "(TagName=\"Data.Damage\")" Damage))
  (GameplayEffects|ApplyGameplayEffectSpecToSelf AC _returnvalue_2))